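; BP_SaveData holds a player's persistent progression and profile: XP, level, unlocked weapons, loadouts, account name and tutorial state.
; SetDefaultValues seeds a fresh profile with a starter rifle and pistol, a matching default loadout and a placeholder name, then returns itself.
; GetCurrentRequiredXP looks up the next level's threshold in the RequiredXP map, with a large fallback when none exists.
; GetReplicatableSaveData packs just the account name into a struct for replication.
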(fn `GetCurrentRequiredXP`
  (returns (RequiredXP :type Integer))
  (bind (_value _returnvalue) (`BlueprintMapLibrary.Map_Find` (`self.RequiredXP`) (+ (`self.Level`) 1)))
  (if _returnvalue
    (return _value)
    (else
      (return 999999))))

(fn `GetReplicatableSaveData`
  (returns (ReplicatedSaveData :type "/Game/Game/Progression/S_ReplicatedSaveData Structure"))
  (return (make `/Game/Game/Progression/S_ReplicatedSaveData` (`self.AccountName`))))

(fn `SetDefaultValues`
  (returns (ReferenceSelf :type "/Game/Game/Progression/BP_SaveData Object Reference"))
  ;[1 1 1] Standaardlevels neerzetten
  (set `self.XP` 0)
  (set `self.Level` 0)
  ;[1 1 1] Standaard weapons unlocked
  (`KismetArrayLibrary.Array_Add` (`self.UnlockedWeapons`) (make `/Game/Game/Progression/SaveDataTypes/S_SaveDataUnlockedWeapon` "automaticrifle"))
  (`KismetArrayLibrary.Array_Add` (`self.UnlockedWeapons`) (make `/Game/Game/Progression/SaveDataTypes/S_SaveDataUnlockedWeapon` "pistol"))
  ;[1 1 1] Default loadout maken
  (`KismetArrayLibrary.Array_Add` (`self.Loadouts`) (make `/Game/Game/Progression/SaveDataTypes/S_SaveDataLoadout` (make `/Game/Game/Progression/SaveDataTypes/S_SaveDataLoadoutWeapon` "automaticrifle") (make `/Game/Game/Progression/SaveDataTypes/S_SaveDataLoadoutWeapon` "pistol")))
  ;[1 1 1] Setup account name
  (set `self.AccountNameSet` false)
  (set `self.AccountName` "Testname")
  (set `self.TutorialPlayed` false)
  (return self))