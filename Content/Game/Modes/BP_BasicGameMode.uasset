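; Base multiplayer game mode that runs FFA or two-team matches with player spawning, deaths and scoring.
; A Tick-driven state machine moves from waiting for full teams through timed play to a win screen, then returns players to the main menu.
; Joining players fill the smallest team, and kills credit the last two attackers with kill and assist.
; Team scores sum player scores; Tick copies match data to GameState, while client calls push player stats.
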(event `self.ReceiveBeginPlay`
  (bind _teams (`self.GenerateTeams`))
  (set `self.Teams` _teams)
  (set `self.CurrentGameState` "NewEnumerator0")
  (set `/Game/Game/Modes/GS_BasicGameState.WinScore` (`self.WinScore`) (cast `/Game/Game/Modes/GS_BasicGameState` (`GameplayStatics.GetGameState`) :!pure true)))

(event `self.ReceiveTick`
  (params (DeltaSeconds :type "Float (single-precision)"))
  (`self.UpdateState` DeltaSeconds)
  (`self.UpdateGameState`))

(event `AfterSpawn`
  (params (Player :type "/Game/FirstPerson/Blueprints/BP_FirstPersonCharacter Object Reference"))
  ;[1 1 1] Wachten totdat teams generate zijn
  (if (not (> (`KismetArrayLibrary.Array_Length` (`self.Teams`)) 0))
    (`KismetSystemLibrary.Delay` 0.2))
  ;[1 1 1] Speler toevoegen aan team
  (`self.AddPlayerToTeam` (`|GetArrayItem` (`self.Teams`) (`self.FindSmallestTeam`)) Player)
  (`self.RespawnPlayer` Player))

(event `CheckPlayerDeath`
  (params (Player :type "/Game/FirstPerson/Blueprints/BP_FirstPersonCharacter Object Reference"))
  ;[1 1 1] Checken of een speler dood is. Zo ja, maken we hem dood
  (if (<= (`/Game/Game/HealthComponent.Health` (`/Game/FirstPerson/Blueprints/BP_FirstPersonCharacter.HealthComponent` Player)) 0)
    (set `/Game/Game/HealthComponent.Dead` true (`/Game/FirstPerson/Blueprints/BP_FirstPersonCharacter.HealthComponent` Player))
    (`self.KillPlayer` Player)))

(event `KillPlayer`
  (params (Player :type "/Game/FirstPerson/Blueprints/BP_FirstPersonCharacter Object Reference"))
  (bind _attacks (`/Game/Game/HealthComponent.Attacks` (`/Game/FirstPerson/Blueprints/BP_FirstPersonCharacter.HealthComponent` Player)))
  (bind _returnvalue (`KismetArrayLibrary.Array_Length` _attacks))
  (bind (_attacker _weapon) (break `/Game/Game/S_Attack` (`|GetArrayItem` _attacks (- _returnvalue 1))))
  (`/Game/FirstPerson/Blueprints/BP_FirstPersonCharacter.HandleRespawn` Player)
  (if (> (`KismetArrayLibrary.Array_Length` _attacks) 1)
    (`self.OnKill` Player _attacker (`.Attacker_2_F733934F45BDE4847F7EA191148A41D9` (break `/Game/Game/S_Attack` (`|GetArrayItem` _attacks (- _returnvalue 2)))) _weapon)
    (else
      (`self.OnKill` Player _attacker null _weapon))))

(event `RespawnPlayer`
  (params (Player :type "/Game/FirstPerson/Blueprints/BP_FirstPersonCharacter Object Reference"))
  (`self.K2_SetActorTransform` Player (`self.GetSpawnpoint` Player) false false))

(event `self.OnKill`
  (params (Killed :type "/Game/FirstPerson/Blueprints/BP_FirstPersonCharacter Object Reference") (Killer :type "/Game/FirstPerson/Blueprints/BP_FirstPersonCharacter Object Reference") (Assister :type "/Game/FirstPerson/Blueprints/BP_FirstPersonCharacter Object Reference") (Weapon :type "/Game/Game/Weapons/S_Weapon Structure"))
  (`self.HandleKill` Killed Killer Assister Weapon))

(event `self.K2_PostLogin`
  (params (NewPlayer :type "PlayerController Object Reference"))
  (`KismetSystemLibrary.Delay` 1.0)
  (`/Game/FirstPerson/Blueprints/BP_FirstPersonCharacter.RequestPersonalPlayerData` (cast `/Game/FirstPerson/Blueprints/BP_FirstPersonCharacter` (`Controller.K2_GetPawn` NewPlayer) :!pure true)))

(event `ReceivePersonalPlayerData`
  (params (Data :type "/Game/Game/Progression/S_ReplicatedSaveData Structure"))
  (`BlueprintMapLibrary.Map_Add` (`self.PlayerNames`) (cast `/Game/FirstPerson/Blueprints/BP_FirstPersonCharacter` (`Controller.K2_GetPawn` (stale `self.K2_PostLogin` NewPlayer)) :!pure true) (`.AccountName_2_A1254CD149632C308BB5B4AB9719C871` (break `/Game/Game/Progression/S_ReplicatedSaveData` Data)))
  (`self.ReplicatePlayerData`))

(event `HandleKill`
  (params (Killed :type "/Game/FirstPerson/Blueprints/BP_FirstPersonCharacter Object Reference") (Killer :type "/Game/FirstPerson/Blueprints/BP_FirstPersonCharacter Object Reference") (Assister :type "/Game/FirstPerson/Blueprints/BP_FirstPersonCharacter Object Reference") (Weapon :type "/Game/Game/Weapons/S_Weapon Structure"))
  (`self.Add Player Data` Killer 1)
  (`/Engine/EditorBlueprintResources/StandardMacros.IsValid` Assister
    (:`Is Valid`
      (`self.Add Player Data` Assister 0 1))))

(fn `Add Player Data`
  (params (Player :type "/Game/FirstPerson/Blueprints/BP_FirstPersonCharacter Object Reference") (Kills :type Integer) (Assists :type Integer) (Score :type Integer))
  (locals (OldData :type "/Game/Game/Modes/S_PlayerGameData Structure"))
  (bind _playersdata (`self.PlayersData`))
  (bind (_kills _assists _score) (break `/Game/Game/Modes/S_PlayerGameData` (`local.OldData`)))
  (set `local.OldData` (`BlueprintMapLibrary.Map_Find` _playersdata Player))
  (`BlueprintMapLibrary.Map_Remove` _playersdata Player)
  (bind _structout (setmembers `/Game/Game/Modes/S_PlayerGameData` :`StructRef` (`local.OldData`) :`Kills` (+ _kills (`local.Kills`)) :`Assists` (+ _assists (`local.Assists`)) :`Score` (+ _score (`local.Score`))))
  (`BlueprintMapLibrary.Map_Add` (`self.PlayersData`) (`local.Player`) _structout)
  (`self.UpdateTeamScores`)
  (`self.ReplicatePlayerData`))

(fn `AddPlayerToTeam`
  (params (Team :type "/Game/Game/Modes/S_GameTeam Structure") (Player :type "/Game/FirstPerson/Blueprints/BP_FirstPersonCharacter Object Reference"))
  (locals (TempMembers :type "Array of /Game/FirstPerson/Blueprints/BP_FirstPersonCharacter Object Reference"))
  (bind _output_get (set `local.TempMembers` (`.TeamMembers_9_29E770F04C7F277B0C7E62AACB0F0DEF` (break `/Game/Game/Modes/S_GameTeam` Team))))
  (`KismetArrayLibrary.Array_Add` _output_get Player)
  (bind _structout (setmembers `/Game/Game/Modes/S_GameTeam` :`StructRef` Team :`TeamMembers` (`local.TempMembers`)))
  (`KismetArrayLibrary.Array_Set` (`self.Teams`) (`self.GetTeamIndex` Team) _structout)
  (`BlueprintMapLibrary.Map_Add` (`self.PlayersData`) (`local.Player`) (make `/Game/Game/Modes/S_PlayerGameData` 0)))

(fn `DebugTeams`
  (for _array_element (`self.Teams`)
    (bind (_teamname _teamcolor _teammembers) (break `/Game/Game/Modes/S_GameTeam` _array_element))
    (`KismetSystemLibrary.PrintString` (`KismetStringLibrary.Concat_StrStr` _teamname " has " (`KismetStringLibrary.Conv_IntToString` (`KismetArrayLibrary.Array_Length` _teammembers)) " players"))))

(fn `FindSmallestTeam`
  (returns (SmallestTeamIndex :type Integer))
  (locals (CurrentSmallestTeam :type "/Game/Game/Modes/S_GameTeam Structure"))
  (set `local.CurrentSmallestTeam` (`|GetArrayItem` (`self.Teams`)))
  (for _array_element (`self.Teams`)
    (if (< (`KismetArrayLibrary.Array_Length` (`.TeamMembers_9_29E770F04C7F277B0C7E62AACB0F0DEF` (break `/Game/Game/Modes/S_GameTeam` _array_element))) (`KismetArrayLibrary.Array_Length` (`.TeamMembers_9_29E770F04C7F277B0C7E62AACB0F0DEF` (break `/Game/Game/Modes/S_GameTeam` (`local.CurrentSmallestTeam`)))))
      (set `local.CurrentSmallestTeam` _array_element)))
  (return (`self.GetTeamIndex` (`local.CurrentSmallestTeam`))))

(fn `GenerateTeams`
  (returns (Teams :type "Array of /Game/Game/Modes/S_GameTeam Structure"))
  (locals (TeamsArray :type "Array of /Game/Game/Modes/S_GameTeam Structure"))
  (`|ExecutionSequence`
    (:`then_0`
      (if (`self.FFA`)
        ;[1 1 1] FFA Teams aanmaken voor het aantal spelers dat er is
        (for _index (range 1 (+ (`self.AmountOfPlayers`) 1))
          (`KismetArrayLibrary.Array_Add` (`local.TeamsArray`) (make `/Game/Game/Modes/S_GameTeam` :`TeamName` (`KismetStringLibrary.Concat_StrStr` "Team " (`KismetStringLibrary.Conv_IntToString` _index)) :`TeamColor` (make `Color` 0 0 255) :`TeamSize` 1)))
        (else
          ;[1 1 1] 2 teams aanmaken voor niet FFA modussen
          (`KismetArrayLibrary.Array_Add` (`local.TeamsArray`) (make `/Game/Game/Modes/S_GameTeam` :`TeamName` "Americans" :`TeamColor` (make `Color` 255) :`TeamSize` 1))
          (`KismetArrayLibrary.Array_Add` (`local.TeamsArray`) (make `/Game/Game/Modes/S_GameTeam` :`TeamName` "Drug" :`TeamColor` (make `Color` 0 0 255) :`TeamSize` 1)))))
    (:`then_1`
      (return (`local.TeamsArray`)))))

(fn `GetCurrentAmountOfPlayers`
  (returns (CurrentAmountOfPlayers :type Integer))
  (locals (CurrentAmount :type Integer))
  (for _array_element (`self.Teams`)
    (set `local.CurrentAmount` (+ (`local.CurrentAmount`) (`KismetArrayLibrary.Array_Length` (`.TeamMembers_9_29E770F04C7F277B0C7E62AACB0F0DEF` (break `/Game/Game/Modes/S_GameTeam` _array_element))))))
  (return (`local.CurrentAmount`)))

(fn `GetPlayerTeam`
  (params (Player :type "/Game/FirstPerson/Blueprints/BP_FirstPersonCharacter Object Reference"))
  (returns (Team :type "/Game/Game/Modes/S_GameTeam Structure"))
  (for _array_element (`self.Teams`)
    (if (`KismetArrayLibrary.Array_Contains` (`.TeamMembers_9_29E770F04C7F277B0C7E62AACB0F0DEF` (break `/Game/Game/Modes/S_GameTeam` _array_element)) Player)
      (return _array_element)))
  (return (`|GetArrayItem` (`self.Teams`))))

(fn `GetSpawnpoint`
  (params (Player :type "/Game/FirstPerson/Blueprints/BP_FirstPersonCharacter Object Reference"))
  (returns (Spawnpoint :type "Transform Structure"))
  (locals (PossibleSpawnLocations :type "Array of Transform Structure"))
  (`|ExecutionSequence`
    (:`then_0`
      (if (`self.FFA`)
        (for _array_element (`/Game/Maps/PDA_GameMap.Spawnpoints` (`self.GameMap`))
          (`KismetArrayLibrary.Array_Add` (`local.PossibleSpawnLocations`) (`.Transform_2_8B58BB04490A52A0AE92ACB11B559C9B` (break `/Game/Maps/S_Spawnpoint` _array_element))))
        (else
          (for _array_element_2 (`/Game/Maps/PDA_GameMap.Spawnpoints` (`self.GameMap`))
            (bind (_transform _team1) (break `/Game/Maps/S_Spawnpoint` _array_element_2))
            (if (== (`self.GetTeamIndex` (`self.GetPlayerTeam` Player)) (`KismetMathLibrary.SelectInt` 0 1 _team1))
              (`KismetArrayLibrary.Array_Add` (`local.PossibleSpawnLocations`) _transform))))))
    (:`then_1`
      (return (`KismetArrayLibrary.Array_Random` (`local.PossibleSpawnLocations`))))))

(fn `GetTeamIndex`
  (params (Team :type "/Game/Game/Modes/S_GameTeam Structure"))
  (returns (Index :type Integer))
  (for (_array_element _array_index) (`self.Teams`)
    (if (`KismetStringLibrary.EqualEqual_StrStr` (`.TeamName_2_51C6E62749BD9D7FEE5F0998813946E6` (break `/Game/Game/Modes/S_GameTeam` _array_element)) (`.TeamName_2_51C6E62749BD9D7FEE5F0998813946E6` (break `/Game/Game/Modes/S_GameTeam` Team)))
      (return _array_index)))
  (return 0))

(fn `GetTotalAmountOfPlayers`
  (returns (CurrentAmountOfPlayers :type Integer))
  (locals (CurrentAmount :type Integer))
  (for _array_element (`self.Teams`)
    (set `local.CurrentAmount` (+ (`local.CurrentAmount`) (`.TeamSize_15_CD7B6E2949F980DC3B82AFB1C1557EB7` (break `/Game/Game/Modes/S_GameTeam` _array_element)))))
  (return (`local.CurrentAmount`)))

(fn `IsWinner`
  (returns (WinnerFound :type Boolean))
  (for _array_element (`self.Teams`)
    (if (>= (`.Score_13_C6C6BE2B4ACF9D0E710F06B6064B4A8F` (break `/Game/Game/Modes/S_GameTeam` _array_element)) (`self.WinScore`))
      (return true)))
  (return false))

(fn `ReplicatePlayerData`
  (locals (Data :type "Array of /Game/Game/Modes/S_ReplicatedPlayerData Structure"))
  (bind _keys (`BlueprintMapLibrary.Map_Keys` (`self.PlayersData`)))
  (for _array_element _keys
    (`KismetArrayLibrary.Array_Add` (`local.Data`) (make `/Game/Game/Modes/S_ReplicatedPlayerData` _array_element (`BlueprintMapLibrary.Map_Find` (`self.PlayersData`) _array_element) (`BlueprintMapLibrary.Map_Find` (`self.PlayerNames`) _array_element))))
  (for _array_element_2 _keys
    (`/Game/FirstPerson/Blueprints/BP_FirstPersonCharacter.CL_UpdateGameState` _array_element_2 (`local.Data`))))

(fn `SendPlayerBack`
  (params (Player :type "/Game/FirstPerson/Blueprints/BP_FirstPersonCharacter Object Reference"))
  (`/Game/FirstPerson/Blueprints/BP_FirstPersonCharacter.SendToMainMenu` Player))

(fn `SendPlayersBack`
  (for _array_element (`self.Teams`)
    (for _array_element_2 (`.TeamMembers_9_29E770F04C7F277B0C7E62AACB0F0DEF` (break `/Game/Game/Modes/S_GameTeam` _array_element))
      (`self.SendPlayerBack` _array_element_2))))

(fn `SetStatePlay`
  (set `self.CurrentGameState` "NewEnumerator1")
  (set `self.PlayingTimeLeft` (`KismetMathLibrary.Conv_IntToDouble` (`self.PlayTimeSeconds`))))

(fn `SetStateWinScreen`
  (set `self.CurrentGameState` "NewEnumerator2")
  (set `self.WinscreenTimeLeft` 10.0))

(fn `SetupPlayerData`
  (params (Player :type "/Game/FirstPerson/Blueprints/BP_FirstPersonCharacter Object Reference"))
  (`BlueprintMapLibrary.Map_Add` (`self.PlayersData`) Player (make `/Game/Game/Modes/S_PlayerGameData` 0)))

(fn `UpdateGameState`
  (bind _asgs_basic_game_state (cast `/Game/Game/Modes/GS_BasicGameState` (`GameplayStatics.GetGameState`) :!pure true))
  (set `/Game/Game/Modes/GS_BasicGameState.CurrentGameTime` (`self.PlayingTimeLeft`) _asgs_basic_game_state)
  (set `/Game/Game/Modes/GS_BasicGameState.CurrentGameState` (`self.CurrentGameState`) _asgs_basic_game_state)
  (set `/Game/Game/Modes/GS_BasicGameState.Teams` (`self.Teams`) _asgs_basic_game_state)
  (set `/Game/Game/Modes/GS_BasicGameState.PlayersData` (`self.PlayersData`) _asgs_basic_game_state))

(fn `UpdateState`
  (params (DeltaTime :type "Float (double-precision)"))
  (if (`self.GameActive`)
    (switch `/Game/Game/Modes/E_GameState` (`self.CurrentGameState`)
      (:`NewEnumerator0`
        ;[1 1 1] Wachten totdat alle spelers gejoined zijn, dan playing starten. NOG SPELERS CINEMATICS ENZO
        (if (== (`self.GetCurrentAmountOfPlayers`) (`self.GetTotalAmountOfPlayers`))
          (`self.SetStatePlay`)))
      (:`NewEnumerator1`
        ;[1 1 1] Normale game, mensen zijn aan het spelen
        ;;[1 1 1] Timer updaten
        (set `self.PlayingTimeLeft` (- (`self.PlayingTimeLeft`) (`local.DeltaTime`)))
        ;;[1 1 1] Als tijd afgelopen of team heeft winscore bereikt, beeindig game
        (if (or (`self.IsWinner`) (<= (`self.PlayingTimeLeft`) 0.0))
          (`self.SetStateWinScreen`)))
      (:`NewEnumerator2`
        ;[1 1 1] Winscherm
        (set `self.WinscreenTimeLeft` (- (`self.WinscreenTimeLeft`) (`local.DeltaTime`)))
        (if (<= (`self.WinscreenTimeLeft`) 0.0)
          (set `self.GameActive` false)
          (`self.SendPlayersBack`))))))

(fn `UpdateTeamScores`
  (locals (CurrentTeamScore :type Integer))
  (for _array_element (`self.Teams`)
    (set `local.CurrentTeamScore` 0)
    (`|ExecutionSequence`
      (:`then_0`
        ;[1 1 1] Totale score van team berekenen
        (for _array_element_2 (`.TeamMembers_9_29E770F04C7F277B0C7E62AACB0F0DEF` (break `/Game/Game/Modes/S_GameTeam` _array_element))
          (set `local.CurrentTeamScore` (+ (`local.CurrentTeamScore`) (`.Score_6_7A52065047B9A7C5C5EF4684B1D1EF94` (break `/Game/Game/Modes/S_PlayerGameData` (`BlueprintMapLibrary.Map_Find` (`self.PlayersData`) _array_element_2)))))))
      (:`then_1`
        ;[1 1 1] Team updaten
        (bind _structout (setmembers `/Game/Game/Modes/S_GameTeam` :`StructRef` _array_element :`Score` (`local.CurrentTeamScore`)))
        (`KismetArrayLibrary.Array_Set` (`self.Teams`) (`self.GetTeamIndex` _array_element) _structout)))))

(fn `UserConstructionScript`)