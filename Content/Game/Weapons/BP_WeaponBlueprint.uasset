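; Weapon actor Blueprint that manages modular attachments on its skeletal mesh and plays a first-person rifle shoot montage.
; PlaceAttachment spawns the attachment's Blueprint, snaps it to the socket named by its type, and records it in SpawnedAttachments.
; Removal looks up that record by type, then destroys the actor and drops the entry.
; RemoveAllAttachments calls this removal while iterating the same array.
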(fn `GetSocketLocation`
  (params (SocketName :type Name))
  (returns (Location :type "Vector Structure"))
  (return (`SceneComponent.GetSocketLocation` (`self.SkeletalMesh`) SocketName)))

(fn `GetSpawnedAttachment`
  (params (AttachmentType :type "/Game/Game/Weapons/Attachments/PDA_Attachment Object Reference"))
  (returns (SpawnedAttachment :type "/Game/Game/Weapons/Attachments/S_SpawnedAttachment Structure"))
  (for _array_element (`self.SpawnedAttachments`)
    (if (== (`/Game/Game/Weapons/Attachments/PDA_Attachment.Type` (`.AttachmentType_2_82606EC04227E038ABD8F1B61A9EEAB0` (break `/Game/Game/Weapons/Attachments/S_SpawnedAttachment` _array_element))) (`local.AttachmentType`))
      (return _array_element))))

(fn `PlaceAttachment`
  (params (Attachment :type "/Game/Game/Weapons/Attachments/PDA_Attachment Object Reference"))
  (bind _returnvalue (`|SpawnActorFromClass` (`/Game/Game/Weapons/Attachments/PDA_Attachment.Blueprint` Attachment) (`SceneComponent.GetSocketTransform` (`self.SkeletalMesh`) (`KismetStringLibrary.Conv_StringToName` (`/Game/Game/Weapons/Attachments/PDA_AttachmentType.SocketName` (`/Game/Game/Weapons/Attachments/PDA_Attachment.Type` (`local.Attachment`)))) "RTS_World") "Undefined" "OverrideRootScale" null null))
  (`self.K2_AttachToComponent` _returnvalue (`self.SkeletalMesh`) (`KismetStringLibrary.Conv_StringToName` (`/Game/Game/Weapons/Attachments/PDA_AttachmentType.SocketName` (`/Game/Game/Weapons/Attachments/PDA_Attachment.Type` (`local.Attachment`)))) "SnapToTarget" "SnapToTarget" "SnapToTarget" true)
  (`KismetArrayLibrary.Array_Add` (`self.SpawnedAttachments`) (make `/Game/Game/Weapons/Attachments/S_SpawnedAttachment` (`local.Attachment`) _returnvalue)))

(fn `PlayShootAnimation`
  (params (FirstPersonCharacter :type "/Game/FirstPerson/Blueprints/BP_FirstPersonCharacter Object Reference"))
  (`AnimInstance.Montage_Play` (`SkeletalMeshComponent.GetAnimInstance` (`/Game/FirstPerson/Blueprints/BP_FirstPersonCharacter.FirstPersonMesh` FirstPersonCharacter)) "/Game/FirstPersonArms/Animations/FP_Rifle_Shoot_Montage.FP_Rifle_Shoot_Montage" 1.0 "MontageLength" 0.0 true))

(fn `RemoveAllAttachments`
  (for _array_element (`self.SpawnedAttachments`)
    (`self.RemoveAttachment` (`.AttachmentType_2_82606EC04227E038ABD8F1B61A9EEAB0` (break `/Game/Game/Weapons/Attachments/S_SpawnedAttachment` _array_element)))))

(fn `RemoveAttachment`
  (params (AttachmentType :type "/Game/Game/Weapons/Attachments/PDA_Attachment Object Reference"))
  (bind _spawnedattachment (`self.GetSpawnedAttachment` AttachmentType))
  (bind (_attachmenttype _attachmentblueprint) (break `/Game/Game/Weapons/Attachments/S_SpawnedAttachment` _spawnedattachment))
  (`/Engine/EditorBlueprintResources/StandardMacros.IsValid` _attachmenttype
    (:`Is Valid`
      (`self.K2_DestroyActor` _attachmentblueprint)
      (`KismetArrayLibrary.Array_RemoveItem` (`self.SpawnedAttachments`) _spawnedattachment))))

(fn `UserConstructionScript`)