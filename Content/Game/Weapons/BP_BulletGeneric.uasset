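; Generic projectile bullet fired by a weapon, which supplies its damage and maximum range.
; It rotates to follow its velocity and records its spawn point in the construction script, destroying itself on Tick once it travels beyond range.
; On hit, the server damages any HealthComponent on the struck actor, crediting the weapon owner, or otherwise attaches a timed bullet-hole decal flagged as replicated, then destroys the bullet.
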(event `self.ReceiveBeginPlay`
  ;[1 1 1] Zorgt ervoor dat de kogel de rotatie volgt van de kant die hij op gaat
  (set `ProjectileMovementComponent.bRotationFollowsVelocity` true (`self.ProjectileMovement`)))

(event `self.ReceiveTick`
  (params (DeltaSeconds :type "Float (single-precision)"))
  ;[1 1 1] Als de kogel verder weg is dan zijn max range, dan despawned hij
  (if (> (`KismetMathLibrary.VSize` (- (`self.K2_GetActorLocation`) (`self.StartPosition`))) (`/Game/Game/Weapons/PDA_WeaponData.Range` (`.WeaponData_2_BFC8D1524617E9E9165547AF5E01466E` (break `/Game/Game/Weapons/S_Weapon` (`self.WeaponShotFrom`)))))
    (`self.K2_DestroyActor`)))

(event `self.ReceiveHit`
  (params (MyComp :type "PrimitiveComponent Object Reference") (Other :type "Actor Object Reference") (OtherComp :type "PrimitiveComponent Object Reference") (bSelfMoved :type Boolean) (HitLocation :type "Vector Structure") (HitNormal :type "Vector Structure") (NormalImpulse :type "Vector Structure") (Hit :type "HitResult Structure (by ref)"))
  (bind _returnvalue (`self.GetComponentByClass` Other "/Game/Game/HealthComponent.HealthComponent_C"))
  ;[1 1 1] Bullet hit detection
  (`/Engine/EditorBlueprintResources/ActorMacros.Switch Has Authority`
    (:`Authority`
      (`|ExecutionSequence`
        (:`then_0`
          (`/Engine/EditorBlueprintResources/StandardMacros.IsValid` _returnvalue
            (:`Is Valid`
              (`/Game/Game/HealthComponent.Damage` :`self` _returnvalue :`Damage` (`/Game/Game/Weapons/PDA_WeaponData.Damage` (`.WeaponData_2_BFC8D1524617E9E9165547AF5E01466E` (break `/Game/Game/Weapons/S_Weapon` (`self.WeaponShotFrom`)))) :`Attacker` (`self.WeaponOwner`)))))
        (:`then_1`
          (`/Engine/EditorBlueprintResources/StandardMacros.IsValid` _returnvalue
            (:`Is Not Valid`
              (bind _returnvalue_2 (`GameplayStatics.SpawnDecalAttached` "/Game/Game/Weapons/Bullet/BulletHoleTexture_Mat.BulletHoleTexture_Mat" (5.0 5.0 5.0) OtherComp "None" HitLocation (`KismetMathLibrary.Conv_VectorToRotator` HitNormal) "KeepWorldPosition" (`self.BulletHoleStayTime`)))
              (`ActorComponent.SetIsReplicated` _returnvalue_2 true))))
        (:`then_2`
          (`self.K2_DestroyActor`))))))

(fn `UserConstructionScript`
  (set `self.StartPosition` (`self.K2_GetActorLocation`)))