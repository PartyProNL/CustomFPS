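; BP_MenuController is the main menu controller, showing the start menu on BeginPlay with the menu input context, save data and mouse cursor.
; It tracks the current widget so Enhanced Input actions can close the start menu or send Back to base pages.
; Tick drives matchmaking updates through BP_GameInstance, and a cancel action clears its matchmaking flag.
; OpenMenu creates and displays a given widget class without removing the previous one.
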(event `self.ReceiveTick`
  (params (DeltaSeconds :type "Float (single-precision)"))
  (`/Game/Game/Progression/BP_GameInstance.UpdateMatchmaking` (cast `/Game/Game/Progression/BP_GameInstance` (`GameplayStatics.GetGameInstance`) :!pure true)))

(event `self.ReceiveBeginPlay`
  (`EnhancedInputSubsystemInterface.AddMappingContext` (subsystem `EnhancedInputLocalPlayerSubsystem`) "/Game/UserInterface/MainMenu/Input/IMC_Menu.IMC_Menu" 0 (struct))
  (bind _returnvalue (`|CreateWidget` "/Game/UserInterface/MainMenu/Pages/WB_StartMenu.WB_StartMenu_C"))
  (bind _output_get (set `self.CurrentMenu` _returnvalue))
  (`UserWidget.AddToViewport` _output_get 0)
  (`/Game/Game/Progression/BP_GameInstance.LoadSaveDataIfNotLoaded` (cast `/Game/Game/Progression/BP_GameInstance` (`GameplayStatics.GetGameInstance`) :!pure true))
  (set `self.bShowMouseCursor` true))

(event `EnhancedInput|/Game/UserInterface/MainMenu/Input/IA_MenuEnter`
  (params (ActionValue :type Boolean) (ElapsedSeconds :type "Float (double-precision)") (TriggeredSeconds :type "Float (double-precision)") (InputAction :type "InputAction Object Reference" :default "/Game/UserInterface/MainMenu/Input/IA_MenuEnter.IA_MenuEnter"))
  (:`Triggered`
    (`|ExecutionSequence`
      (:`then_0`
        (bind _aswb_start_menu (cast `/Game/UserInterface/MainMenu/Pages/WB_StartMenu` (`self.CurrentMenu`)))
        (`/Game/UserInterface/MainMenu/Pages/WB_StartMenu.CloseMenu` _aswb_start_menu)))))

(event `EnhancedInput|/Game/UserInterface/MainMenu/Input/IA_CancelMatchmaking`
  (params (ActionValue :type Boolean) (ElapsedSeconds :type "Float (double-precision)") (TriggeredSeconds :type "Float (double-precision)") (InputAction :type "InputAction Object Reference" :default "/Game/UserInterface/MainMenu/Input/IA_CancelMatchmaking.IA_CancelMatchmaking"))
  (:`Triggered`
    (set `/Game/Game/Progression/BP_GameInstance.CurrentlyMatchmaking` false (cast `/Game/Game/Progression/BP_GameInstance` (`GameplayStatics.GetGameInstance`) :!pure true))))

(event `EnhancedInput|/Game/UserInterface/MainMenu/Input/IA_MenuBack`
  (params (ActionValue :type Boolean) (ElapsedSeconds :type "Float (double-precision)") (TriggeredSeconds :type "Float (double-precision)") (InputAction :type "InputAction Object Reference" :default "/Game/UserInterface/MainMenu/Input/IA_MenuBack.IA_MenuBack"))
  (:`Triggered`
    (bind _aswb_base_page (cast `/Game/UserInterface/MainMenu/Pages/Default/WB_BasePage` (`self.CurrentMenu`)))
    (`/Game/UserInterface/MainMenu/Pages/Default/WB_BasePage.OnBack` _aswb_base_page)))

(fn `OpenMenu`
  (params (NewParam :type "UserWidget Class Reference"))
  (bind _returnvalue (`|CreateWidget` NewParam))
  (bind _output_get (set `self.CurrentMenu` _returnvalue))
  (`UserWidget.AddToViewport` _output_get 0))

(fn `UserConstructionScript`)